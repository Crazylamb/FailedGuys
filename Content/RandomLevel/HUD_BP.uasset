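; HUD Blueprint that shows the game's time, score and level, plus a Game Over message.
; On BeginPlay it casts the game mode to GameMode_BP and caches it.
; Each DrawHUD pass draws the game mode's values as text along the top, with level displayed one lower than stored.
; When GameOver is set, it draws the message and also calls the game mode's Restart from inside the draw event.
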(event EventBeginPlay
  (bind _asgame_mode_bp (Utilities|Casting|CastToGameMode_BP (Game|GetGameMode)))
  (Variables|Default|SetGamemode _asgame_mode_bp))

(event EventDrawHUD
  (params (SizeX :type Integer) (SizeY :type Integer))
  (bind _gamemode (Variables|Default|GetGamemode))
  (HUD|DrawText (Utilities|String|BuildString(Integer) "Time: " "" (Variables|/Game/RandomLevel/GameMode_BP.GameMode_BP_C|GetTime (Variables|Default|GetGamemode))) "(R=0.005208,G=0.000526,B=0.001307,A=1.000000)" 1e+01 1e+01 0 3.0 false)
  (HUD|DrawText (Utilities|String|BuildString(Integer) "Score: " "" (Math|Conversions|ToInteger(Byte) (Variables|/Game/RandomLevel/GameMode_BP.GameMode_BP_C|GetScore (Variables|Default|GetGamemode)))) "(R=0.005208,G=0.000526,B=0.001307,A=1.000000)" 2e+02 1e+01 0 3.0 false)
  (HUD|DrawText (Utilities|String|BuildString(Integer) "Level: " "" (- (Variables|/Game/RandomLevel/GameMode_BP.GameMode_BP_C|GetLevel (Variables|Default|GetGamemode)) 1)) "(R=0.005208,G=0.000526,B=0.001307,A=1.000000)" 4e+02 1e+01 0 3.0 false)
  (if (Variables|/Game/RandomLevel/GameMode_BP.GameMode_BP_C|GetGameOver _gamemode)
    (HUD|DrawText "Game Over" "(R=0.984375,G=0.000000,B=0.164252,A=1.000000)" 4.5e+02 3.5e+02 0 5.0 false)
    (Default|Restart _gamemode)))

(fn ConstructionScript)