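; Game mode for a randomly generated level game, holding score, time, level and game-over state.
; A StartGame macro resets that state and starts a looping one-second Clock timer, which raises Level about every half minute up to a cap.
; BeginPlay and Additionallvls call Generation on the RandomLevelGen actor.
; RestartGame only reruns StartGame, while Restart reloads the current map after a short delay.
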(event Custom|Restart%20Game
  (Utilities|StartGame))

(event Custom|Clock
  (Variables|Default|SetTime (+ (Variables|Default|GetTime) 1))
  (if (and (== (Math|Integer|%(Integer) (Variables|Default|GetTime) 31) 30) (< (Variables|Default|GetLevel) 7))
    (Variables|Default|SetLevel (+ (Variables|Default|GetLevel) 1))))

(event Custom|Additional%20lvls
  (bind _returnvalue (Actor|GetActorOfClass "/Game/RandomLevel/RandomLevelGen.RandomLevelGen_C"))
  (Default|Generation _returnvalue))

(event Custom|Restart
  (Utilities|FlowControl|Delay 1.0)
  (bind _returnvalue (Game|GetCurrentLevelName true))
  (Game|OpenLevel(byName) (Utilities|String|StringToName _returnvalue)))

(event EventBeginPlay
  (Utilities|StartGame
    (:out
      (bind _returnvalue (Actor|GetActorOfClass "/Game/RandomLevel/RandomLevelGen.RandomLevelGen_C"))
      (Default|Generation _returnvalue))))

(event EventTick
  (params (DeltaSeconds :type Float%20%28single-precision%29)))

(fn ConstructionScript)