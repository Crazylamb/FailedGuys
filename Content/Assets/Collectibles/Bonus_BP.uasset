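; Cupcake bonus collectible that temporarily lets things pass through actors of the configured classes.
; On BeginPlay it randomly either shows the cupcake or destroys itself, surviving about one time in five.
; Any actor overlap hides it and switches those actors' collision to Walkthrough.
; A five-second Delay inside the loop then leads to restoring BlockAllDynamic, with DestroyActor called inside that restore loop.
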(event EventBeginPlay
  (Rendering|SetVisibility (Variables|Default|GetCupcake) false false)
  (if (>= (Math|Random|RandomInteger 10) 8)
    (Rendering|SetVisibility (Variables|Default|GetCupcake) true false)
    (else
      (Actor|DestroyActor))))

(event Collision|EventActorBeginOverlap
  (params (OtherActor :type Actor%20Object%20Reference))
  (Rendering|SetVisibility (Variables|Default|GetCupcake) false false)
  (for _array_element (Variables|Default|GetActor%20Class)
    (bind _outactors (Actor|GetAllActorsOfClass _array_element))
    (for _array_element_2 _outactors
      (Collision|SetCollisionProfileName (Actor|GetComponentbyClass _array_element_2 "/Script/Engine.PrimitiveComponent") "Walkthrough" true :!class /Script/Engine.PrimitiveComponent)
      (Utilities|FlowControl|Delay 5.0)
      (for _array_element_3 (Variables|Default|GetActor%20Class)
        (bind _outactors_2 (Actor|GetAllActorsOfClass _array_element_3))
        (for _array_element_4 _outactors_2
          (Collision|SetCollisionProfileName (Actor|GetComponentbyClass _array_element_4 "/Script/Engine.PrimitiveComponent") "BlockAllDynamic" true :!class /Script/Engine.PrimitiveComponent)
          (Actor|DestroyActor))))))

(event EventTick
  (params (DeltaSeconds :type Float%20%28single-precision%29)))

(fn ConstructionScript)

(fn TurnonCollisions)