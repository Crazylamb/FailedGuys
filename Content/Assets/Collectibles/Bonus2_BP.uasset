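; Collectible apple bonus that randomly appears at level start and temporarily drops the game mode's Level to 1 when overlapped.
; On BeginPlay a random roll either shows the apple or destroys the actor.
; Any actor overlap hides the apple and saves Level and Time from GameMode_BP.
; After a short delay it restores both saved values, rewinding Time to the pickup moment, then destroys itself.
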(event EventBeginPlay
  (Rendering|SetVisibility (Variables|Default|GetApple) false false)
  (if (>= (Math|Random|RandomInteger 10) 6)
    (Rendering|SetVisibility (Variables|Default|GetApple) true false)
    (else
      (Actor|DestroyActor))))

(event Collision|EventActorBeginOverlap
  (params (OtherActor :type Actor%20Object%20Reference))
  (Rendering|SetVisibility (Variables|Default|GetApple) false false)
  (bind _asgame_mode_bp (Utilities|Casting|CastToGameMode_BP (Game|GetGameMode)))
  (bind _output_get (Variables|Default|SetLevelNum (Variables|/Game/RandomLevel/GameMode_BP.GameMode_BP_C|GetLevel _asgame_mode_bp)))
  (bind _output_get_2 (Variables|Default|SetTimer (Variables|/Game/RandomLevel/GameMode_BP.GameMode_BP_C|GetTime _asgame_mode_bp)))
  (Variables|/Game/RandomLevel/GameMode_BP.GameMode_BP_C|SetLevel _asgame_mode_bp 1)
  (Utilities|FlowControl|Delay 5.0)
  (Variables|/Game/RandomLevel/GameMode_BP.GameMode_BP_C|SetLevel _asgame_mode_bp _output_get)
  (Variables|/Game/RandomLevel/GameMode_BP.GameMode_BP_C|SetTime _asgame_mode_bp _output_get_2)
  (Actor|DestroyActor))

(fn ConstructionScript)