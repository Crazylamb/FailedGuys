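; Rotation_Bp is an actor that swings back and forth around its roll axis, faster at higher game levels.
; Each Tick adds Speed times GameMode_BP's Level, scaled by delta time, to the roll while keeping pitch and yaw.
; Speed flips sign when roll reaches plus or minus Angle in the direction of travel, so the direction check prevents repeated flipping past the limit.
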(event Collision|EventActorBeginOverlap
  (params (OtherActor :type Actor%20Object%20Reference)))

(event EventTick
  (params (DeltaSeconds :type Float%20%28single-precision%29))
  (bind _returnvalue (Transformation|GetActorRotation))
  (bind _angle (Variables|Default|GetAngle))
  ;[1 1 1] Changing rotation for an object
  (bind _asgame_mode_bp (Utilities|Casting|CastToGameMode_BP (Game|GetGameMode)))
  (if (or (and (>= (.roll _returnvalue) _angle) (> (Variables|Default|GetSpeed) 0.0)) (and (<= (.roll _returnvalue) (* _angle -1.0)) (< (Variables|Default|GetSpeed) 0.0)))
    (Variables|Default|SetSpeed (* -1 (Variables|Default|GetSpeed))))
  (Transformation|SetActorRotation (Math|Rotator|MakeRotator (+ (.roll _returnvalue) (* DeltaSeconds (* (Variables|/Game/RandomLevel/GameMode_BP.GameMode_BP_C|GetLevel _asgame_mode_bp) (Variables|Default|GetSpeed)))) (.pitch _returnvalue) (.yaw _returnvalue))))

(fn ConstructionScript)